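; Clickable door Blueprint that alternately swings open and closed by 45 degrees of yaw.
; BeginPlay enables mouse click events, and each click on the Door component flips between OpenDoor and CloseDoor through a FlipFlop, unless an animation is running.
; Each event drives a timeline-based rotator lerp; opening starts from zero rotation, while closing starts from the current rotation.
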(event OnClicked(Door)
  (params (TouchedComponent :type Primitive%20Component%20Object%20Reference) (ButtonPressed :type Key%20Structure :default "None"))
  ;[1 1 1] A partir du clic, lancer la fonction ouvrir
  (Development|PrintString "Hello")
  (if (not (Variables|Default|GetanimationGoing))
    (Utilities|FlowControl|FlipFlop
      (:A
        (CallFunction|OpenDoor))
      (:B
        (CallFunction|CloseDoor)))))

(event Custom|OpenDoor
  ;[1 1 1] Ouvrir la porte selon un angle de rotation
  (Variables|Default|SetanimationGoing true)
  (Variables|Default|SetRelative%20Rotation (Variables|/Script/Engine.SceneComponent|GetRelativeRotation (Variables|Default|Getdoor)))
  (bind _dooralpha (Timeline|Timeline PlayFromStart)
    (:Update
      (Transformation|SetRelativeRotation (Variables|Default|Getdoor) (Math|Rotator|Lerp(Rotator) "0, 0, 0" (Math|Rotator|Delta(Rotator) (Variables|Default|GetRelative%20Rotation) "0.000000,-45.000000,0.000000") _dooralpha) false false))
    (:Finished
      (Variables|Default|SetanimationGoing false))))

(event Custom|CloseDoor
  ;[1 1 1] Fermer la porte selon un angle de rotation
  (Variables|Default|SetanimationGoing true)
  (Variables|Default|SetRelative%20Rotation (Variables|/Script/Engine.SceneComponent|GetRelativeRotation (Variables|Default|Getdoor)))
  (bind _dooralpha (Timeline|Timeline_0 PlayFromStart)
    (:Update
      (Transformation|SetRelativeRotation (Variables|Default|Getdoor) (Math|Rotator|Lerp(Rotator) (Variables|Default|GetRelative%20Rotation) (Math|Rotator|Delta(Rotator) (Variables|Default|GetRelative%20Rotation) "0.000000,45.000000,0.000000") _dooralpha) false false))
    (:Finished
      (Variables|Default|SetanimationGoing false))))

(event EventBeginPlay
  ;[1 1 1] activer events clics
  (Variables|/Script/Engine.PlayerController|SetbEnableClickEvents (Game|GetPlayerController 0) true))

(fn ConstructionScript)